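; BP_FightingCrunch is a pawn Blueprint that fires a projectile on left mouse click.
; Each press spawns a BP_Projectile at the ProjectileSpawnPosition component's world transform, ignoring collisions at the spawn point.
; A HealthComponent is present but unused in the graph, and the construction script only calls its parent.
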(event EventBeginPlay
  (|CallParentFunction) ; This node is disabled and will not be called.\nDrag off pins to build functionality.
)

(event Collision|EventActorBeginOverlap
  (params (OtherActor :type Actor%20Object%20Reference))
  (|CallParentFunction OtherActor) ; This node is disabled and will not be called.\nDrag off pins to build functionality.
)

(event EventTick
  (params (DeltaSeconds :type Float%20%28single-precision%29))
  (|CallParentFunction DeltaSeconds) ; This node is disabled and will not be called.\nDrag off pins to build functionality.
)

(event Input|MouseEvents|LeftMouseButton
  (params (Key :type Key%20Structure :default "None"))
  (:Pressed
    (Game|SpawnActorfromClass "/Game/Actors/BP_Projectile.BP_Projectile_C" (Transformation|GetWorldTransform (Variables|Default|GetProjectileSpawnPosition)) "AlwaysSpawn" "MultiplyWithRoot" 0 0)))

(fn ConstructionScript
  (|CallParentFunction))